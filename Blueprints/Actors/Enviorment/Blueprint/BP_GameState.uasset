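; Game state Blueprint that runs the day/night cycle by driving the time of day on the level's BP_SunSky actor.
; BeginPlay caches that actor and starts a looping timer at a configurable tick rate.
; Each tick advances a seconds counter, converts it through a timespan offset to start at 8:00, and writes the SunSky's hours, minutes and seconds.
; The counter resets after a full day.
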(event Custom|TimeUpdate
  ;[1 1 1] Cycle Day/Night
  (bind _output_get (Variables|Default|SetTimeOfDayInSeconds (+ (Variables|Default|GetTimeOfDayInSeconds) (Variables|Default|GetAmountOfSecondsToAddPerTick))))
  (Variables|/Game/00_app/Blueprints/Actors/Enviorment/Blueprint/BP_SunSky.BP_SunSky_C|SetHours (Variables|Default|GetSun%20Sky) (.Hours (Math|Timespan|BreakTimespan (Math|Timespan|MakeTimespan 0 8 0 _output_get))))
  (Variables|/Game/00_app/Blueprints/Actors/Enviorment/Blueprint/BP_SunSky.BP_SunSky_C|SetMinutes (Variables|Default|GetSun%20Sky) (.Minutes (Math|Timespan|BreakTimespan (Math|Timespan|MakeTimespan 0 8 0 _output_get))))
  (Variables|/Game/00_app/Blueprints/Actors/Enviorment/Blueprint/BP_SunSky.BP_SunSky_C|SetSeconds (Variables|Default|GetSun%20Sky) (.Seconds (Math|Timespan|BreakTimespan (Math|Timespan|MakeTimespan 0 8 0 _output_get))))
  (if (>= (Variables|Default|GetTimeOfDayInSeconds) 86400)
    (Variables|Default|SetTimeOfDayInSeconds 0)))

(event EventBeginPlay
  ;[1 1 1] Cycle Day/Night
  (bind _returnvalue (Actor|GetActorOfClass "/Game/00_app/Blueprints/Actors/Enviorment/Blueprint/BP_SunSky.BP_SunSky_C"))
  (bind _asbp_sun_sky (Utilities|Casting|CastToBP_SunSky _returnvalue))
  (Variables|Default|SetSun%20Sky _asbp_sun_sky)
  (Utilities|Time|SetTimerbyEvent (delegate Custom|TimeUpdate) (/ 1.0 (Variables|Default|GetAmountToTickASecond)) true))

(fn ConstructionScript)
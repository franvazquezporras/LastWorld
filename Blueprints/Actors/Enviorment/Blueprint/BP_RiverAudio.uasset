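; BP_RiverAudio is an actor that keeps a river sound cue at the point on its spline nearest the player's selector.
; On BeginPlay it caches the player character as a BP_Selector reference.
; A self-calling event with a short delay then moves the audio component to that closest spline point, raised slightly on Z, so the sound follows along the river.
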(event Custom|Move%20Audio
  (bind _spline (Variables|Default|GetSpline))
  (bind _selector (Variables|Default|GetSelector))
  (bind _returnvalue (Transformation|GetActorLocation _selector))
  (bind _returnvalue_2 (Spline|FindLocationClosesttoWorldLocation _spline _returnvalue "World"))
  (Transformation|SetWorldLocation (Variables|Default|GetRiver_cue) (Math|Vector|MakeVector (.x _returnvalue_2) (.y _returnvalue_2) (+ (.z _returnvalue_2) 5e+01)) false false)
  (Utilities|FlowControl|Delay 0.05)
  (CallFunction|MoveAudio))

(event EventBeginPlay
  (CallFunction|GetPlayer)
  (CallFunction|MoveAudio))

(fn ConstructionScript)

(fn GetPlayer
  (Variables|Default|GetSelector
    (:then
      _)
    (:else
      (bind _asbp_selector (Utilities|Casting|CastToBP_Selector (Game|GetPlayerCharacter 0)))
      (Variables|Default|SetSelector _asbp_selector)))
  (return (Variables|Default|GetSelector)))
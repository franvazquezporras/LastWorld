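; BP_ManaZone is a single-use mana pickup that restores a fixed amount of mana to the player character that touches it.
; On box overlap it casts to BP_PlayerCharacter, adds to CurrentMana clamped at MaxMana, tells the HUD to refresh the mana display, then destroys itself.
; GetHudREF lazily fetches BP_Player_HUD from the first player controller and caches it for reuse.
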(event OnComponentBeginOverlap(Box)
  (params (OverlappedComponent :type Primitive%20Component%20Object%20Reference) (OtherActor :type Actor%20Object%20Reference) (OtherComp :type Primitive%20Component%20Object%20Reference) (OtherBodyIndex :type Integer) (bFromSweep :type Boolean) (SweepResult :type Hit%20Result%20Structure%20%28by%20ref%29))
  (bind _asbp_player_character (Utilities|Casting|CastToBP_PlayerCharacter OtherActor))
  (if (>= (+ (Variables|/Game/00_app/Blueprints/Characters/PlayerCharacter/Blueprint/BP_PlayerCharacter.BP_PlayerCharacter_C|GetCurrentMana _asbp_player_character) 1e+01) (Variables|/Game/00_app/Blueprints/Characters/PlayerCharacter/Blueprint/BP_PlayerCharacter.BP_PlayerCharacter_C|GetMaxMana _asbp_player_character))
    (Variables|/Game/00_app/Blueprints/Characters/PlayerCharacter/Blueprint/BP_PlayerCharacter.BP_PlayerCharacter_C|SetCurrentMana _asbp_player_character (Variables|/Game/00_app/Blueprints/Characters/PlayerCharacter/Blueprint/BP_PlayerCharacter.BP_PlayerCharacter_C|GetMaxMana _asbp_player_character))
    (else
      (Variables|/Game/00_app/Blueprints/Characters/PlayerCharacter/Blueprint/BP_PlayerCharacter.BP_PlayerCharacter_C|SetCurrentMana _asbp_player_character (+ (Variables|/Game/00_app/Blueprints/Characters/PlayerCharacter/Blueprint/BP_PlayerCharacter.BP_PlayerCharacter_C|GetCurrentMana _asbp_player_character) 1e+01))))
  (bind _as_bp_player_hud (CallFunction|GetHudREF))
  (Default|RefreshPlayerMana _as_bp_player_hud)
  (Actor|DestroyActor))

(fn ConstructionScript)

(fn GetHudREF
  ;[1 1 1] Get Player HUD Reference
  (Variables|Default|GetBp%20Player%20HUD
    (:then
      _)
    (:else
      (bind _asbp_player_hud (Utilities|Casting|CastToBP_Player_HUD (HUD|GetHUD (Game|GetPlayerController 0))))
      (Variables|Default|SetBp%20Player%20HUD _asbp_player_hud)))
  (return (Variables|Default|GetBp%20Player%20HUD)))
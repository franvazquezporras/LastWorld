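; BP_Key is a key pickup actor that gives a key to the player who picks it up.
; It overrides the parent's PickIt event, running the parent logic first and then casting the picker to BP_PlayerCharacter.
; On a successful cast it calls AddKey with its KeyType, and all other events are left to the parent.
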(event EventBeginPlay
  (|CallParentFunction) ; This node is disabled and will not be called.\nDrag off pins to build functionality.
)

(event Collision|EventActorBeginOverlap
  (params (OtherActor :type Actor%20Object%20Reference))
  (|CallParentFunction OtherActor) ; This node is disabled and will not be called.\nDrag off pins to build functionality.
)

(event EventTick
  (params (DeltaSeconds :type Float%20%28single-precision%29))
  (|CallParentFunction DeltaSeconds) ; This node is disabled and will not be called.\nDrag off pins to build functionality.
)

(event EventPickIt
  (params (ActorWhoPickIt :type Actor%20Object%20Reference))
  ;[1 1 1] Add the key to player
  (|CallParentFunction ActorWhoPickIt)
  (bind _asbp_player_character (Utilities|Casting|CastToBP_PlayerCharacter ActorWhoPickIt))
  (Default|AddKey _asbp_player_character (Variables|Default|GetKeyType)))

(fn ConstructionScript
  (|CallParentFunction))
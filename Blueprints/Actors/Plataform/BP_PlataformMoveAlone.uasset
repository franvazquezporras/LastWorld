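; Moving platform actor that travels back and forth along a spline on its own from BeginPlay.
; The MovePlatform timeline scales its TravelDistance track by spline length to set the mesh's world location.
; Each update also reapplies the spline's starting roll and yaw with zero pitch, so orientation does not follow the curve.
; When the timeline finishes, the Invertir flag flips and the Reverse event plays it backward or from the start.
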(event Custom|Reverse
  (bind _spline (Variables|Default|GetSpline))
  (bind _returnvalue (Spline|GetRotationatDistanceAlongSpline _spline 0.0 "Local"))
  (if (Variables|Default|GetInvertir)
    (bind _traveldistance (Timeline|MovePlatform Reverse)
      (:Update
        (Transformation|SetWorldLocation (Variables|Default|GetStaticMesh) (Spline|GetLocationatDistanceAlongSpline _spline (* _traveldistance (Spline|GetSplineLength (Variables|Default|GetSpline))) "World") false false)
        (Transformation|SetRelativeRotation (Variables|Default|GetStaticMesh) (Math|Rotator|MakeRotator (.roll _returnvalue) 0.0 (.yaw _returnvalue)) false false))
      (:Finished
        (Variables|Default|SetInvertir (not (Variables|Default|GetInvertir)))
        (CallFunction|Reverse)))
    (else
      (Timeline|MovePlatform PlayFromStart))))

(event EventBeginPlay
  (bind _spline (Variables|Default|GetSpline))
  (bind _spline_2 (Variables|Default|GetSpline))
  (bind _returnvalue (Spline|GetRotationatDistanceAlongSpline _spline 0.0 "Local"))
  (bind _returnvalue_2 (Spline|GetRotationatDistanceAlongSpline _spline_2 0.0 "Local"))
  (Transformation|SetRelativeRotation (Variables|Default|GetStaticMesh) (Math|Rotator|MakeRotator (.roll _returnvalue_2) 0.0 (.yaw _returnvalue_2)) false false)
  (bind _traveldistance (Timeline|MovePlatform Play)
    (:Update
      (Transformation|SetWorldLocation (Variables|Default|GetStaticMesh) (Spline|GetLocationatDistanceAlongSpline _spline (* _traveldistance (Spline|GetSplineLength (Variables|Default|GetSpline))) "World") false false)
      (Transformation|SetRelativeRotation (Variables|Default|GetStaticMesh) (Math|Rotator|MakeRotator (.roll _returnvalue) 0.0 (.yaw _returnvalue)) false false))
    (:Finished
      (Variables|Default|SetInvertir (not (Variables|Default|GetInvertir)))
      (CallFunction|Reverse))))

(fn ConstructionScript)
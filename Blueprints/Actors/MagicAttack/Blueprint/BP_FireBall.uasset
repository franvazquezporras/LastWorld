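; BP_FireBall is a magic attack actor that damages what it overlaps and has a short lifetime.
; On overlap with an actor that can be damaged, it applies randomly selected damage, plays a 2D impact sound and destroys itself.
; A delay started on BeginPlay destroys it if it has not hit anything.
; The random index never reaches the last of the damage options.
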(event EventBeginPlay
  ;[1 1 1] LifeTime
  (Utilities|FlowControl|Delay 3.0)
  (if (not (Game|IsActorBeingDestroyed))
    (Actor|DestroyActor)))

(event Collision|EventActorBeginOverlap
  (params (OtherActor :type Actor%20Object%20Reference))
  ;[1 1 1] Impact with enemy
  (if (Variables|/Script/Engine.Actor|GetbCanBeDamaged OtherActor)
    (Game|Damage|ApplyDamage OtherActor (Utilities|Select :Index (Math|Random|RandomInteger 5) :Option%200 0.8 :Option%201 0.1 :Option%202 0.25 :Option%203 0.5 :Option%204 1.0 :Option%205 0.75) 0 self)
    (Audio|PlaySound2D "/Game/00_app/Sounds/Steps/ImpactFireBall.ImpactFireBall" 1.0 1.0 0.0 0 0)
    (Actor|DestroyActor)))

(fn ConstructionScript)
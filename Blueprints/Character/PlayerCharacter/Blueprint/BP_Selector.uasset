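; Level-select player character that travels between LevelPads along LevelPath splines.
; Forward/right input picks a path from the overlapped pad, then a timeline plays or reverses, feeding spline tangents into movement input at a rate scaled by walk speed and spline length.
; DoOnce gates lock input during travel, and arrival resets them and shows the HeadsUpLevel info hidden on departure.
; It also toggles the pause menu, backing out of its options submenu first.
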(event Custom|ReachedDestination
  (bind _hub (Variables|Default|GetHub))
  ;[1 1 1] Selector level movement
  (Default|DisplayLevelInfo (Variables|Default|GetHub))
  (Variables|Default|SetCurrentLevelPath 0)
  (Utilities|FlowControl|Sequence
    (:then_0
      (Utilities|FlowControl|DoOnce false) ; enters at Reset
    )
    (:then_1
      (Utilities|FlowControl|DoOnce false) ; enters at Reset
    )))

(event EventBeginPlay
  ;[1 1 1] Active widget for first level
  (bind _returnvalue (UserInterface|CreateWidget "/Game/00_app/Widgets/SelectorLevelUI/HeadsUpLevel.HeadsUpLevel_C"))
  (bind _output_get (Variables|Default|SetHub _returnvalue))
  (UserInterface|Viewport|AddtoViewport _output_get 0)
  (CallFunction|ReachedDestination))

(event Input|ActionEvents|InputActionPausetheGame
  (params (Key :type Key%20Structure :default "None"))
  (bind _returnvalue (Game|GetPlayerController 0))
  ;[1 1 1] Open/Close Pause Menu
  (:Pressed
    (Variables|Default|GetPauseMenuREF
      (:then
        _)
      (:else
        (bind _returnvalue_2 (UserInterface|CreateWidget "/Game/00_app/Widgets/PauseMenu/WBP_PauseMenu.WBP_PauseMenu_C"))
        (Variables|Default|SetPauseMenuREF _returnvalue_2)))
    (if (UserInterface|Viewport|IsinViewport (Variables|Default|GetPauseMenuREF))
      (if (UserInterface|Viewport|IsinViewport (Variables|/Game/00_app/Widgets/PauseMenu/WBP_PauseMenu.WBP_PauseMenu_C|GetOptionMenuPauseREF (Variables|Default|GetPauseMenuREF)))
        (Widget|RemovefromParent (Variables|/Game/00_app/Widgets/PauseMenu/WBP_PauseMenu.WBP_PauseMenu_C|GetOptionMenuPauseREF (Variables|Default|GetPauseMenuREF)))
        (Widget|SetVisibility (Variables|Default|GetPauseMenuREF) "Visible")
        (else
          (Widget|RemovefromParent (Variables|Default|GetPauseMenuREF))
          (Game|SetGamePaused false)
          (Variables|/Script/Engine.PlayerController|SetbShowMouseCursor _returnvalue false)
          (Input|SetInputModeGameOnly _returnvalue)))
      (else
        (UserInterface|Viewport|AddtoViewport (Variables|Default|GetPauseMenuREF) 0)
        (Game|SetGamePaused true)
        (Variables|/Script/Engine.PlayerController|SetbShowMouseCursor _returnvalue true)
        (Input|SetInputModeGameandUI _returnvalue (Variables|Default|GetPauseMenuREF) "LockInFullscreen" false)))))

(event Input|AxisEvents|InputAxisMoveForward
  (params (AxisValue :type Float%20%28single-precision%29))
  (bind _currentlevelpath (Variables|Default|GetCurrentLevelPath))
  (bind _currentlevelpath_2 (Variables|Default|GetCurrentLevelPath))
  (bind _spline (Variables|/Game/00_app/Blueprints/Actors/LevelSelector/Blueprint/LevelPath.LevelPath_C|GetSpline _currentlevelpath))
  ;[1 1 1] Selector level movement
  (if (!= AxisValue 0.0)
    (Utilities|FlowControl|DoOnce false
      (:Completed
        (Default|HideLevelInfo (Variables|Default|GetHub))
        (bind _levelpad (CallFunction|GetCurrentLevel))
        (bind _aslevel_pad (Utilities|Casting|CastToLevelPad _levelpad))
        (CallFunction|GetLevelPad _aslevel_pad AxisValue true)
        (if (> (Input|AxisValues|GetMoveForward) 0.0)
          (Variables|Default|SetScale%20Value 1.0)
          (CallFunction|SetPlayRate)
          (Utilities|IsValid _currentlevelpath_2
            (:Is%20Valid
              (bind _pathdistance (Timeline|TimeMovement PlayFromStart)
                (:Update
                  (Pawn|Input|AddMovementInput (Math|Vector|Normalize (Spline|GetTangentatDistanceAlongSpline _spline (* _pathdistance (Spline|GetSplineLength _spline)) "World")) (Variables|Default|GetScale%20Value) false))
                (:Finished
                  (CallFunction|ReachedDestination :!label _label))))
            (:Is%20Not%20Valid
              (goto _label)))
          (else
            (Variables|Default|SetScale%20Value -1.0)
            (CallFunction|SetPlayRate)
            (Utilities|IsValid _currentlevelpath_2
              (:Is%20Valid
                (Timeline|TimeMovement ReverseFromEnd))
              (:Is%20Not%20Valid
                (goto _label)))))))))

(event Input|AxisEvents|InputAxisMoveRight
  (params (AxisValue :type Float%20%28single-precision%29))
  (bind _currentlevelpath (Variables|Default|GetCurrentLevelPath))
  (bind _currentlevelpath_2 (Variables|Default|GetCurrentLevelPath))
  (bind _spline (Variables|/Game/00_app/Blueprints/Actors/LevelSelector/Blueprint/LevelPath.LevelPath_C|GetSpline _currentlevelpath))
  ;[1 1 1] Selector level movement
  (if (!= AxisValue 0.0)
    (Utilities|FlowControl|DoOnce false
      (:Completed
        (Default|HideLevelInfo (Variables|Default|GetHub))
        (bind _levelpad (CallFunction|GetCurrentLevel))
        (bind _aslevel_pad (Utilities|Casting|CastToLevelPad _levelpad))
        (CallFunction|GetLevelPad _aslevel_pad AxisValue false)
        (if (> (Input|AxisValues|GetMoveRight) 0.0)
          (Variables|Default|SetScale%20Value 1.0)
          (CallFunction|SetPlayRate)
          (Utilities|IsValid _currentlevelpath_2
            (:Is%20Valid
              (bind _pathdistance (Timeline|TimeMovement PlayFromStart)
                (:Update
                  (Pawn|Input|AddMovementInput (Math|Vector|Normalize (Spline|GetTangentatDistanceAlongSpline _spline (* _pathdistance (Spline|GetSplineLength _spline)) "World")) (Variables|Default|GetScale%20Value) false))
                (:Finished
                  (CallFunction|ReachedDestination :!label _label))))
            (:Is%20Not%20Valid
              (goto _label)))
          (else
            (Variables|Default|SetScale%20Value -1.0)
            (CallFunction|SetPlayRate)
            (Utilities|IsValid _currentlevelpath_2
              (:Is%20Valid
                (Timeline|TimeMovement ReverseFromEnd))
              (:Is%20Not%20Valid
                (goto _label)))))))))

(fn ConstructionScript)

(fn GetAnimBPREF
  ;[1 1 1] Get Anim Reference
  (Variables|Default|GetAnimREF
    (:then
      _)
    (:else
      (bind _asabp_player (Utilities|Casting|CastToABP_Player (Components|SkeletalMesh|GetAnimInstance (Variables|Character|GetMesh))))
      (Variables|Default|SetAnimREF _asabp_player)))
  (return (Variables|Default|GetAnimREF)))

(fn GetCurrentLevel
  (return (Utilities|Array|Get(acopy) (Collision|GetOverlappingActors "/Game/00_app/Blueprints/Actors/LevelSelector/Blueprint/LevelPad.LevelPad_C" :!class /Script/Engine.Actor))))

(fn GetLevelPad
  (params (LevelPad :type Level%20Pad%20Object%20Reference) (AxisValue :type Float%20%28double-precision%29) (IsMoveForwards :type Boolean))
  (if IsMoveForwards
    (bind _aslevel_path (Utilities|Casting|CastToLevelPath (Utilities|SelectObject (Variables|/Game/00_app/Blueprints/Actors/LevelSelector/Blueprint/LevelPad.LevelPad_C|GetPathUp LevelPad) (Variables|/Game/00_app/Blueprints/Actors/LevelSelector/Blueprint/LevelPad.LevelPad_C|GetPathDown LevelPad) (> AxisValue 0.0))))
    (Variables|Default|SetCurrentLevelPath _aslevel_path)
    (else
      (bind _aslevel_path_2 (Utilities|Casting|CastToLevelPath (Utilities|SelectObject (Variables|/Game/00_app/Blueprints/Actors/LevelSelector/Blueprint/LevelPad.LevelPad_C|GetPathRight LevelPad) (Variables|/Game/00_app/Blueprints/Actors/LevelSelector/Blueprint/LevelPad.LevelPad_C|GetPathLeft LevelPad) (> AxisValue 0.0))))
      (Variables|Default|SetCurrentLevelPath _aslevel_path_2))))

(fn SetPlayRate
  (bind _currentlevelpath (Variables|Default|GetCurrentLevelPath))
  (Utilities|IsValid _currentlevelpath
    (:Is%20Valid
      (Components|Timeline|SetPlayRate (Variables|Default|GetTimeMovement) (/ (Variables|/Script/Engine.CharacterMovementComponent|GetMaxWalkSpeed (Variables|Character|GetCharacterMovement)) (Spline|GetSplineLength (Variables|/Game/00_app/Blueprints/Actors/LevelSelector/Blueprint/LevelPath.LevelPath_C|GetSpline _currentlevelpath)))))))
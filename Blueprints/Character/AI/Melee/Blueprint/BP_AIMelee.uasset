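; BP_AIMelee is a melee zombie enemy that attacks the player, takes damage and dies.
; It binds itself to a health bar widget, refreshed on each hit, and at zero health plays death effects before destroying itself.
; AIBasicAttack plays a montage whose notify fires a sphere trace from the right hand.
; The trace reports a damage sense event and deals randomly chosen damage to BP_PlayerCharacter.
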(event EventBeginPlay
  ;[1 1 1] Control HealthBar
  (bind _asui_enemy_bar (Utilities|Casting|CastToUI_EnemyBar (UserInterface|GetUserWidgetObject (Variables|Default|GetHealthBar))))
  (bind _output_get (Variables|Default|SetEnemyWidgetBar _asui_enemy_bar))
  (Variables|/Game/00_app/Blueprints/Characters/AI/Melee/UI/UI_EnemyBar.UI_EnemyBar_C|SetEnemy _output_get self)
  (Default|UpdateHealth _asui_enemy_bar))

(event Game|Damage|EventAnyDamage
  (params (Damage :type Float%20%28single-precision%29) (DamageType :type Damage%20Type%20Object%20Reference) (InstigatedBy :type Controller%20Object%20Reference) (DamageCauser :type Actor%20Object%20Reference))
  ;[1 1 1] Get Damage
  (if (not (Variables|Default|GetIsDead))
    (Variables|Default|SetHealth (- (Variables|Default|GetHealth) Damage))
    (Default|UpdateHealth (Variables|Default|GetEnemyWidgetBar))
    (if (<= (Variables|Default|GetHealth) 0.0)
      (Pawn|Components|CharacterMovement|DisableMovement (Variables|Character|GetCharacterMovement))
      (Variables|Default|SetIsDead true)
      (Animation|PlayAnimMontage "/Game/00_app/Blueprints/Characters/AI/Melee/Animation/AI_Death.AI_Death" 1.0 "None")
      (Audio|PlaySound2D "/Game/00_app/Sounds/Steps/ZombieDeath.ZombieDeath" 1.0 1.0 0.0 0 0)
      (Utilities|FlowControl|Delay 5.0)
      (Actor|DestroyActor))))

(event EventAIBasicAttack
  (bind _mesh (Variables|Character|GetMesh))
  (bind _returnvalue (Transformation|GetSocketLocation _mesh "hand_RSocket"))
  ;[1 1 1] Attack
  (if (not (Variables|Default|GetIsDead))
    (Animation|Montage|PlayMontage (Variables|Character|GetMesh) "/Game/00_app/Blueprints/Characters/AI/Melee/Animation/Corpse_Alert_Attack_Basic01_Montage.Corpse_Alert_Attack_Basic01_Montage" 2.0
      (:OnNotifyBegin
        (bind _outhit (Collision|SphereTraceByChannel _returnvalue (+ _returnvalue (* (Math|Vector|GetForwardVector (Transformation|GetActorRotation)) 5e+01)) 5e+01 "TraceTypeQuery2" false 0 "None"))
        (Class|AISenseDamage|ReportDamageEvent (.hitactor _outhit) self 1.0 (.tracestart _outhit) "0, 0, 0" "None")
        (bind _asbp_player_character (Utilities|Casting|CastToBP_PlayerCharacter (.hitactor _outhit)))
        (Game|Damage|ApplyDamage _asbp_player_character (Utilities|Select :Index (Math|Random|RandomInteger 4) :Option%200 1e+01 :Option%201 2e+01 :Option%202 15.0 :Option%203 25.0 :Option%204 5.0) 0 0)
        (Audio|PlaySound2D "/Game/00_app/Sounds/Steps/EnemyHit.EnemyHit" 1.0 1.0 0.0 0 0)))))

(fn ConstructionScript)
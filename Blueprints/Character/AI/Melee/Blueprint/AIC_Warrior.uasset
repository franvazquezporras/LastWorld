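; AI controller for the melee Warrior enemy that runs BT_Warrior and feeds its blackboard.
; BeginPlay seeds patrol loop, direction, wait time and death state from the controlled BP_AIMelee and its patrol path.
; Perception updates for the player go to ControlSenses, which tells senses apart by stimulus array index.
; The first sets CanSeePlayer; successful second or third stimuli set IsSearching and TargetLocation, the second also playing a mob sound.
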(event OnPerceptionUpdated(AIPerception)
  (params (UpdatedActors :type Array%20of%20Actor%20Object%20References))
  (for _array_element UpdatedActors
    (bind _asbp_player_character (Utilities|Casting|CastToBP_PlayerCharacter _array_element))
    (bind _info (Class|AIPerceptionComponent|GetActorsPerception (Variables|Default|GetAIPerception) _asbp_player_character))
    (CallFunction|ControlSenses (.lastsensedstimuli _info))))

(event EventBeginPlay
  (bind _returnvalue (AI|GetBlackboard 0))
  (AI|RunBehaviorTree "/Game/00_app/Blueprints/Characters/AI/Melee/Blueprint/BehaviorTree/BT_Warrior.BT_Warrior")
  (bind _asbp_aimelee (Utilities|Casting|CastToBP_AIMelee (Pawn|GetControlledPawn)))
  (bind _output_get (Variables|Default|SetMyPawn _asbp_aimelee))
  (AI|Components|Blackboard|SetValueasBool _returnvalue (Utilities|Name|MakeLiteralName "PathLooping") (Variables|/Game/00_app/Blueprints/Characters/AI/Melee/Blueprint/BP_PatrolPath.BP_PatrolPath_C|GetIsLooping (Variables|/Game/00_app/Blueprints/Characters/AI/Melee/Blueprint/BP_AIMelee.BP_AIMelee_C|GetPatrolPath _output_get)))
  (Class|BlackboardComponent|SetValueasInt _returnvalue (Utilities|Name|MakeLiteralName "Direction") 1)
  (AI|Components|Blackboard|SetValueasFloat _returnvalue (Utilities|Name|MakeLiteralName "WaitTime") (Variables|/Game/00_app/Blueprints/Characters/AI/Melee/Blueprint/BP_PatrolPath.BP_PatrolPath_C|GetWaitTime (Variables|/Game/00_app/Blueprints/Characters/AI/Melee/Blueprint/BP_AIMelee.BP_AIMelee_C|GetPatrolPath (Variables|Default|GetMyPawn))))
  (AI|Components|Blackboard|SetValueasBool _returnvalue (Utilities|Name|MakeLiteralName "IsIADead") (Variables|/Game/00_app/Blueprints/Characters/AI/Melee/Blueprint/BP_AIMelee.BP_AIMelee_C|GetIsDead (Variables|Default|GetMyPawn))))

(event EventTick
  (params (DeltaSeconds :type Float%20%28single-precision%29)))

(fn ConstructionScript)

(fn ControlSenses
  (params (Array :type Array%20of%20AI%20Stimulus%20Structures))
  (for (_array_element _array_index) Array
    (LocalVariables|SetLocalSense _array_element)
    (switch int _array_index
      (:0
        (AI|Components|Blackboard|SetValueasBool (AI|GetBlackboard 0) (Utilities|Name|MakeLiteralName "CanSeePlayer") (.bsuccessfullysensed (LocalVariables|GetLocalSense))))
      (:1
        (if (.bsuccessfullysensed (LocalVariables|GetLocalSense))
          (Audio|PlaySoundatLocation "/Game/00_app/Sounds/Steps/mobSound.mobSound" (.receiverlocation (LocalVariables|GetLocalSense)) "0, 0, 0" 1.0 1.0 0.0 0 0 0 0)
          (AI|Components|Blackboard|SetValueasBool (AI|GetBlackboard 0) (Utilities|Name|MakeLiteralName "IsSearching") (.bsuccessfullysensed (LocalVariables|GetLocalSense)) :!label _label)
          (AI|Components|Blackboard|SetValueasVector (AI|GetBlackboard 0) (Utilities|Name|MakeLiteralName "TargetLocation") (.stimuluslocation (LocalVariables|GetLocalSense)))))
      (:2
        (if (.bsuccessfullysensed (LocalVariables|GetLocalSense))
          (goto _label))))))
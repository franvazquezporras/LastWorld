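; GM_LastWorld is the game mode that handles player respawning and the win screen.
; On BeginPlay it binds to the destroyed event of the player's BP_PlayerCharacter.
; When that character is destroyed, it waits briefly, spawns and possesses a replacement at CheckpointTransform, then rebinds through Respawn so the cycle repeats.
; WinGame creates WBP_WinPanel and adds it to the viewport.
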(event Custom|WinGame
  (bind _returnvalue (UserInterface|CreateWidget "/Game/00_app/Widgets/WBP_WinPanel.WBP_WinPanel_C"))
  (UserInterface|Viewport|AddtoViewport _returnvalue 0))

(event Custom|OnDestroyed_
  (params (DestroyedActor :type Actor%20Object%20Reference))
  (Utilities|FlowControl|Delay 3.0)
  (bind _returnvalue (Game|SpawnActorfromClass "/Game/00_app/Blueprints/Characters/PlayerCharacter/Blueprint/BP_PlayerCharacter.BP_PlayerCharacter_C" (Variables|Default|GetCheckpointTransform) "Undefined" 0 0))
  (Pawn|Possess (Game|GetPlayerController 0) _returnvalue)
  (CallFunction|Respawn))

(event Custom|Respawn
  (bind _asbp_player_character (Utilities|Casting|CastToBP_PlayerCharacter (Game|GetPlayerCharacter 0)))
  (Game|BindEventtoOnDestroyed _asbp_player_character (delegate Custom|OnDestroyed_)))

(event EventBeginPlay
  (bind _asbp_player_character (Utilities|Casting|CastToBP_PlayerCharacter (Game|GetPlayerCharacter 0)))
  (Game|BindEventtoOnDestroyed _asbp_player_character (delegate Custom|OnDestroyed_)))

(fn ConstructionScript)
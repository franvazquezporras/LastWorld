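; BP_Goal is the level goal, triggered when the player character overlaps its Box.
; On overlap it tells GM_LastWorld the game is won, unlocks progression, then opens BaseLevel after a short delay.
; Unlocking matches the current level name to set flags on the GI_SavedVariable game instance, cached at BeginPlay, with Level 3 also unlocking the bonus level.
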(event OnComponentBeginOverlap(Box)
  (params (OverlappedComponent :type Primitive%20Component%20Object%20Reference) (OtherActor :type Actor%20Object%20Reference) (OtherComp :type Primitive%20Component%20Object%20Reference) (OtherBodyIndex :type Integer) (bFromSweep :type Boolean) (SweepResult :type Hit%20Result%20Structure%20%28by%20ref%29))
  ;[1 1 1] EndLevel, Load next
  (Utilities|Casting|CastToBP_PlayerCharacter OtherActor)
  (bind _asgm_last_world (Utilities|Casting|CastToGM_LastWorld (Game|GetGameMode)))
  (Default|WinGame _asgm_last_world)
  (CallFunction|UnlockNextLevel)
  (Utilities|FlowControl|Delay 3.0)
  (Game|OpenLevel(byObjectReference) "/Game/00_app/Levels/BaseLevel.BaseLevel"))

(event EventBeginPlay
  (CallFunction|GetInstanceREF))

(fn ConstructionScript)

(fn UnlockNextLevel
  (bind _unlockedlevelsref (Variables|Default|GetUnlockedLevelsREF))
  (bind _returnvalue (Game|GetCurrentLevelName true))
  (switch string _returnvalue
    (:Default
      _)
    (:Level1
      (Variables|/Game/00_app/Blueprints/Core/FrameWork/GI_SavedVariable.GI_SavedVariable_C|SetLevel2Unlocked _unlockedlevelsref true))
    (:Level2
      (Variables|/Game/00_app/Blueprints/Core/FrameWork/GI_SavedVariable.GI_SavedVariable_C|SetLevel3Unlocked _unlockedlevelsref true))
    (:Level3
      (Variables|/Game/00_app/Blueprints/Core/FrameWork/GI_SavedVariable.GI_SavedVariable_C|SetLevel4Unlocked _unlockedlevelsref true)
      (Variables|/Game/00_app/Blueprints/Core/FrameWork/GI_SavedVariable.GI_SavedVariable_C|SetLevelBonusUnlocked _unlockedlevelsref true))
    (:Level4
      (Variables|/Game/00_app/Blueprints/Core/FrameWork/GI_SavedVariable.GI_SavedVariable_C|SetLevel5Unlocked _unlockedlevelsref true)))
  (return))

(fn GetInstanceREF
  (Variables|Default|GetUnlockedLevelsREF
    (:then
      _)
    (:else
      (bind _asgi_saved_variable (Utilities|Casting|CastToGI_SavedVariable (Game|GetGameInstance)))
      (Variables|Default|SetUnlockedLevelsREF _asgi_saved_variable)))
  (return (Variables|Default|GetUnlockedLevelsREF)))
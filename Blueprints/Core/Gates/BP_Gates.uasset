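; Key-locked forcefield gate that opens when a player character carrying the correct key overlaps its collision.
; On BeginPlay it creates a dynamic material instance on the forcefield mesh.
; On overlap, a gameplay tag query checks the player's keys; a match disables forcefield collision and plays a timeline driving material opacity.
; UseKey runs on every timeline update with a fixed blue key tag, independent of the CorrectKey query.
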(event OnComponentBeginOverlap(GateCollision)
  (params (OverlappedComponent :type Primitive%20Component%20Object%20Reference) (OtherActor :type Actor%20Object%20Reference) (OtherComp :type Primitive%20Component%20Object%20Reference) (OtherBodyIndex :type Integer) (bFromSweep :type Boolean) (SweepResult :type Hit%20Result%20Structure%20%28by%20ref%29))
  ;[1 1 1] Look For Keys Gate and Open gate
  (bind _asbp_player_character (Utilities|Casting|CastToBP_PlayerCharacter OtherActor))
  (if (GameplayTags|DoesContainerMatchTagQuery (Variables|/Game/00_app/Blueprints/Characters/PlayerCharacter/Blueprint/BP_PlayerCharacter.BP_PlayerCharacter_C|GetNumberOfKeys _asbp_player_character) (Variables|Default|GetCorrectKey))
    (Collision|SetCollisionEnabled (Variables|Default|GetSM_Large_Gate_Forcefield) "NoCollision")
    (bind _newopacity (Timeline|T_Opacity Play)
      (:Update
        (Rendering|Material|SetScalarParameterValue (Variables|Default|GetForceDynamicMaterial) "Opacity" _newopacity :!class /Script/Engine.MaterialInstanceDynamic)
        (Default|UseKey _asbp_player_character "(TagName=\"Key.Blue\")")))))

(event EventBeginPlay
  ;[1 1 1] Get initial material from gate
  (bind _returnvalue (Rendering|Material|CreateDynamicMaterialInstance (Variables|Default|GetSM_Large_Gate_Forcefield) 0 "/Game/00_app/Blueprints/Actors/Architecture/Materials/MI_forcefield.MI_forcefield" "None" :!class /Script/Engine.PrimitiveComponent))
  (Variables|Default|SetForceDynamicMaterial _returnvalue))

(event Collision|EventActorBeginOverlap
  (params (OtherActor :type Actor%20Object%20Reference)))

(event EventTick
  (params (DeltaSeconds :type Float%20%28single-precision%29)))

(fn ConstructionScript)